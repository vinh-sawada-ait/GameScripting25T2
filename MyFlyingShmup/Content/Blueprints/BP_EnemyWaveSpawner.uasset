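; Enemy wave spawner that runs the waves defined in a data asset in order, then shows the HUD end screen.
; Each wave starts on a timer, then spawns its members sequentially after individual delays, passing pickup-drop settings to each enemy by message.
; After the last spawn, it polls every second, pruning invalid enemies from its list, and advances once the list is empty.
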(event `NextWave`
  (bind _result (`/Engine/EditorBlueprintResources/StandardMacros.IncrementInt` (`self.CurrentWaveIndex`))
    (:`  `
      (bind _setofwaves (`/Game/Framework/PDA_SetOfWaves.SetOfWaves` (stale `self.ReceiveBeginPlay` _wavedataasset)))
      (if (`KismetArrayLibrary.Array_IsValidIndex` _setofwaves _result)
        (bind (_output_enemymembers _output_initialwavedelay) (break `/Game/Framework/S_Wave` (`|GetArrayItem` _setofwaves (`self.CurrentWaveIndex`))))
        (`KismetSystemLibrary.K2_SetTimerDelegate` (delegate `StartWave`) _output_initialwavedelay :!label _label)
        (`KismetSystemLibrary.PrintString` "Waiting For Wave")
        (else
          (message `/Game/Framework/BPI_myFlyingShmup.ShowEndScreen` (`PlayerController.GetHUD` (`GameplayStatics.GetPlayerController` 0)) true))))))

(event `self.ReceiveBeginPlay`
  (bind _wavedataasset (`self.WaveDataAsset`)
    (:`then`
      (goto _label))
    (:`else`)))

(event `StartWave`
  (bind _output_enemymembers (break `/Game/Framework/S_Wave` (`|GetArrayItem` (`/Game/Framework/PDA_SetOfWaves.SetOfWaves` (`self.WaveDataAsset`)) (`self.CurrentWaveIndex`))))
  (bind (_output_waveid _output_initialspawndelay _output_enemyclass _output_spawntransform _output_shoulddroppickup _output_pickupclass) (break `/Game/Framework/S_WaveEnemyMember` (`|GetArrayItem` _output_enemymembers (`self.EnemyMemberIndex`))))
  (`KismetSystemLibrary.PrintString` "Starting Wave")
  (bind _output_get (set `self.EnemyMemberIndex` 0))
  (if (> _output_get (`KismetArrayLibrary.Array_LastIndex` _output_enemymembers)) :!label _label_2
    ; Remove any invalid enemies on our list
    (for (_array_element _array_index) (`self.SpawnedEnemies`) :!label _label_3
      (`/Engine/EditorBlueprintResources/StandardMacros.IsValid` _array_element
        (:`Is Not Valid`
          (`KismetArrayLibrary.Array_Remove` (`self.SpawnedEnemies`) _array_index))))
    ; Check if list is empty
    (if (`KismetArrayLibrary.Array_IsEmpty` (`self.SpawnedEnemies`))
      (`self.NextWave`)
      (else
        (`KismetSystemLibrary.Delay` 1.0)
        (goto _label_3)))
    (else
      (`KismetSystemLibrary.PrintString` "Waiting For Next Enemy To Spawn")
      (`KismetSystemLibrary.Delay` _output_initialspawndelay)
      (bind _returnvalue (`|SpawnActorFromClass` _output_enemyclass _output_spawntransform "AlwaysSpawn" "MultiplyWithRoot" null null))
      (message `/Game/Framework/BPI_myFlyingShmup.AssignSpawnedEnemyProps` _returnvalue _output_shoulddroppickup _output_pickupclass)
      (`KismetArrayLibrary.Array_Add` (`self.SpawnedEnemies`) _returnvalue)
      (`/Engine/EditorBlueprintResources/StandardMacros.IncrementInt` (`self.EnemyMemberIndex`)
        (:`  `
          (goto _label_2))))))

(fn `UserConstructionScript`)